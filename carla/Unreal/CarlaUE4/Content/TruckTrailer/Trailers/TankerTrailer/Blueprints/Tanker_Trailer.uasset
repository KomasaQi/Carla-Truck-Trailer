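; Tanker trailer that mirrors the player truck's lights and flags itself to an overlapping truck as attachable.
; The construction script creates dynamic material instances for side lights, both blinkers and brake.
; While ActiveLight is set, Tick polls the player Truck's flags to drive those materials and the brake light intensities, pulsing blinkers through a timeline; otherwise it resets them.
; DetectTruck overlap toggles the truck's TankerTrailer flag and prints an attach prompt on entry.
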(event `self.ReceiveTick`
  (params (DeltaSeconds :type "Float (single-precision)"))
  (bind _brake (`self.Brake`))
  (bind _side_lights (`self.Side_lights`))
  (`|ExecutionSequence`
    (:`then_0`
      (if (`self.Active_Light`)
        (`|ExecutionSequence`
          (:`then_0`
            ;[0.9973 1 0.355] Blinkers
            (bind (_direction _newtrack_1) (`Timeline|Timeline_0` :!label _label)
              (:`Update`
                (bind _astruck (cast `/Game/TruckTrailer/Truck/Blueprints/Truck` (`GameplayStatics.GetPlayerPawn` 0)))
                (`|ExecutionSequence`
                  (:`then_0`
                    (if (`self.F`)
                      (if (`/Game/TruckTrailer/Truck/Blueprints/Truck.LR_Blinker_Trailer` _astruck)
                        (`|ExecutionSequence`
                          (:`then_0`
                            (`MaterialInstanceDynamic.SetScalarParameterValue` (`self.R_Blinker`) "Light" _newtrack_1 :!label _label_2))
                          (:`then_1`
                            (`MaterialInstanceDynamic.SetScalarParameterValue` (`self.L_Blinker`) "Light" _newtrack_1 :!label _label_3)))
                        (else
                          (`|ExecutionSequence`
                            (:`then_0`
                              (`MaterialInstanceDynamic.SetScalarParameterValue` (`self.R_Blinker`) "Light" 1.0 :!label _label_4))
                            (:`then_1`
                              (`MaterialInstanceDynamic.SetScalarParameterValue` (`self.L_Blinker`) "Light" 1.0 :!label _label_5)))))))
                  (:`then_1`
                    (if (`self.Z`)
                      (if (`/Game/TruckTrailer/Truck/Blueprints/Truck.L_Blinker_Trailer` _astruck)
                        (goto _label_3)
                        (else
                          (`|ExecutionSequence`
                            (:`then_0`
                              (goto _label_4))
                            (:`then_1`
                              (goto _label_5)))))))
                  (:`then_2`
                    (if (`self.X`)
                      (if (`/Game/TruckTrailer/Truck/Blueprints/Truck.R_Blinker_Trailer` _astruck)
                        (goto _label_2)
                        (else
                          (`|ExecutionSequence`
                            (:`then_0`
                              (goto _label_4))
                            (:`then_1`
                              (goto _label_5)))))))))))
          (:`then_1`
            ;[1 1 1] Side_Lights
            (bind _astruck_2 (cast `/Game/TruckTrailer/Truck/Blueprints/Truck` (`GameplayStatics.GetPlayerPawn` 0)))
            (if (`/Game/TruckTrailer/Truck/Blueprints/Truck.ActiveLightTrailer` _astruck_2)
              (`MaterialInstanceDynamic.SetScalarParameterValue` _side_lights "Light" 0.0)
              (else
                (`MaterialInstanceDynamic.SetScalarParameterValue` _side_lights "Light" 1.0 :!label _label_6))))
          (:`then_2`
            ;[0.195 0.09652 0.09652] Brake
            (bind _astruck_3 (cast `/Game/TruckTrailer/Truck/Blueprints/Truck` (`GameplayStatics.GetPlayerPawn` 0)))
            (if (`/Game/TruckTrailer/Truck/Blueprints/Truck.Brake_Trailer` _astruck_3)
              (`MaterialInstanceDynamic.SetVectorParameterValue` _brake "Brake" (make `LinearColor` 10.0))
              (`LightComponent.SetIntensity` (`self.R_Brake_Light`) 1000.0)
              (`LightComponent.SetIntensity` (`self.L_Brake_Light`) 1000.0)
              (elif (`/Game/TruckTrailer/Truck/Blueprints/Truck.Light_ON_Trailer` _astruck_3)
                (`MaterialInstanceDynamic.SetVectorParameterValue` (`self.Brake`) "Brake" (make `LinearColor` 0.5))
                (`LightComponent.SetIntensity` (`self.R_Brake_Light`) 250.0)
                (`LightComponent.SetIntensity` (`self.L_Brake_Light`) 250.0)
                (else
                  (`MaterialInstanceDynamic.SetVectorParameterValue` _brake "Brake" (make `LinearColor` 0.0) :!label _label_7)
                  (`LightComponent.SetIntensity` (`self.R_Brake_Light`) 0.0)
                  (`LightComponent.SetIntensity` (`self.L_Brake_Light`) 0.0))))))
        (else
          (`|ExecutionSequence`
            (:`then_0`
              (goto _label_6))
            (:`then_1`
              (goto _label_4))
            (:`then_2`
              (goto _label :!via `SetNewTime`))
            (:`then_3`
              (goto _label_4))
            (:`then_4`
              (goto _label_5))
            (:`then_5`
              (goto _label_7))))))
    (:`then_1`
      ;[0.9648 1 0.5348] Control_Matching
      (bind _astruck_4 (cast `/Game/TruckTrailer/Truck/Blueprints/Truck` (`GameplayStatics.GetPlayerPawn` 0)))
      (`|ExecutionSequence`
        (:`then_0`
          (set `self.F` (`/Game/TruckTrailer/Truck/Blueprints/Truck.LR_Blinker_Trailer` _astruck_4)))
        (:`then_1`
          (set `self.Z` (`/Game/TruckTrailer/Truck/Blueprints/Truck.L_Blinker_Trailer` _astruck_4)))
        (:`then_2`
          (set `self.X` (`/Game/TruckTrailer/Truck/Blueprints/Truck.R_Blinker_Trailer` _astruck_4)))))))

(event `self.DetectTruck.OnComponentBeginOverlap`
  (params (OverlappedComponent :type "PrimitiveComponent Object Reference") (OtherActor :type "Actor Object Reference") (OtherComp :type "PrimitiveComponent Object Reference") (OtherBodyIndex :type Integer) (bFromSweep :type Boolean) (SweepResult :type "HitResult Structure (by ref)"))
  ;[1 1 1] DetectTruck
  (bind _astruck (cast `/Game/TruckTrailer/Truck/Blueprints/Truck` OtherActor))
  (set `/Game/TruckTrailer/Truck/Blueprints/Truck.TankerTrailer` true _astruck)
  (`KismetSystemLibrary.PrintString` "Attach Press \"T\""))

(event `self.DetectTruck.OnComponentEndOverlap`
  (params (OverlappedComponent :type "PrimitiveComponent Object Reference") (OtherActor :type "Actor Object Reference") (OtherComp :type "PrimitiveComponent Object Reference") (OtherBodyIndex :type Integer))
  ;[1 1 1] DetectTruck
  (bind _astruck (cast `/Game/TruckTrailer/Truck/Blueprints/Truck` OtherActor))
  (set `/Game/TruckTrailer/Truck/Blueprints/Truck.TankerTrailer` false _astruck))

(fn `UserConstructionScript`
  (bind _mesh (`self.Mesh`))
  (`|ExecutionSequence`
    (:`then_0`
      (bind _returnvalue (`PrimitiveComponent.CreateDynamicMaterialInstance` _mesh 4 "/Game/TruckTrailer/Trailers/TankerTrailer/Materials/M_Side_light_Inst.M_Side_light_Inst" "None"))
      (set `self.Side_lights` _returnvalue))
    (:`then_1`
      (bind _returnvalue_2 (`PrimitiveComponent.CreateDynamicMaterialInstance` _mesh 5 "/Game/TruckTrailer/Trailers/TankerTrailer/Materials/M_Tanker_Blinker_L_Inst.M_Tanker_Blinker_L_Inst" "None"))
      (set `self.L_Blinker` _returnvalue_2))
    (:`then_2`
      (bind _returnvalue_3 (`PrimitiveComponent.CreateDynamicMaterialInstance` _mesh 6 "/Game/TruckTrailer/Trailers/TankerTrailer/Materials/M_Tanker_Blinker_R_Inst.M_Tanker_Blinker_R_Inst" "None"))
      (set `self.R_Blinker` _returnvalue_3))
    (:`then_3`
      (bind _returnvalue_4 (`PrimitiveComponent.CreateDynamicMaterialInstance` _mesh 1 "/Game/TruckTrailer/Trailers/TankerTrailer/Materials/M_Brake_Tanker_Inst.M_Brake_Tanker_Inst" "None"))
      (set `self.Brake` _returnvalue_4))))